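; Game mode that populates the world with random loot at BeginPlay.
; GenerateItems caches probability totals and row names from DataTables, then spawns a BP_ItemGroup at each DT_ItemGroupLocation row.
; Each group rolls an item count, distinct item types (rerolling duplicates) and an ID per type via cumulative-percent weighted picks.
; The matching BP_WorldItem subclasses spawn at the group's random transforms, initialized with their IDs.
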(event `self.ReceiveBeginPlay`
  (`self.GenerateItems`))

(fn `GenerateItems`
  (locals (ItemGroupRef :type "/Game/Blueprints/Items/BP_ItemGroup Object Reference") (SpawnTransforms :type "Array of Transform Structure") (ItemTypeArray :type "Array of /Game/Blueprints/Datas/Enum/Item/E_ItemType Enum") (SpawnItemArray :type "Array of /Game/Blueprints/Datas/Struct/ItemGeneration/ST_SpawnItem Structure") (ItemType :type "/Game/Blueprints/Datas/Enum/Item/E_ItemType Enum") (SpawnId :type Name) (NumberProbability :type "/Game/Blueprints/Datas/Struct/ItemGeneration/ST_ProbabilityInfo Structure") (SumPercent :type Integer) (ItemTypeProbability :type "/Game/Blueprints/Datas/Struct/ItemGeneration/ST_ProbabilityInfo Structure") (ItemIdProbability :type "Map of /Game/Blueprints/Datas/Enum/Item/E_ItemType Enum to /Game/Blueprints/Datas/Struct/ItemGeneration/ST_ProbabilityInfo Structure"))
  (`|ExecutionSequence`
    (:`then_0`
      (set `local.SumPercent` 0)
      ; 각 숫자가 나올 확률 정보
      (bind _outrownames (`DataTableFunctionLibrary.GetDataTableRowNames` "/Game/Blueprints/Datas/DataTable/ItemGeneration/DT_NumberProbability.DT_NumberProbability"))
      (for _array_element _outrownames
        (bind _returnvalue (`|GetDataTableRow` "/Game/Blueprints/Datas/DataTable/ItemGeneration/DT_NumberProbability.DT_NumberProbability" _array_element)
          (:`then`
            (set `local.SumPercent` (+ (`local.SumPercent`) (`.Percent_10_98C4C114460AC2A5B6C6139E6052683E` (break `/Game/Blueprints/Datas/Struct/ItemGeneration/ST_NumberProbability` _returnvalue)))))))
      (set `local.NumberProbability` (make `/Game/Blueprints/Datas/Struct/ItemGeneration/ST_ProbabilityInfo` (`local.SumPercent`) _outrownames)))
    (:`then_1`
      (set `local.SumPercent` 0)
      ; 각 아이템타입 정보 및 확률
      (bind _outrownames_2 (`DataTableFunctionLibrary.GetDataTableRowNames` "/Game/Blueprints/Datas/DataTable/ItemGeneration/DT_ItemTypeProbability.DT_ItemTypeProbability"))
      (for _array_element_2 _outrownames_2
        (bind _returnvalue_2 (`|GetDataTableRow` "/Game/Blueprints/Datas/DataTable/ItemGeneration/DT_ItemTypeProbability.DT_ItemTypeProbability" _array_element_2)
          (:`then`
            (set `local.SumPercent` (+ (`local.SumPercent`) (`.Percent_4_0DD76C4F406C51CD7E91A680B042B4A1` (break `/Game/Blueprints/Datas/Struct/ItemGeneration/ST_ItemTypeProbability` _returnvalue_2)))))))
      (set `local.ItemTypeProbability` (make `/Game/Blueprints/Datas/Struct/ItemGeneration/ST_ProbabilityInfo` (`local.SumPercent`) _outrownames_2)))
    (:`then_2`
      (set `local.SumPercent` 0)
      ; Ammo가 나올 확률 정보
      (bind _outrownames_3 (`DataTableFunctionLibrary.GetDataTableRowNames` "/Game/Blueprints/Datas/DataTable/ItemGeneration/DT_AmmoProbability.DT_AmmoProbability"))
      (for _array_element_3 _outrownames_3
        (bind _returnvalue_3 (`|GetDataTableRow` "/Game/Blueprints/Datas/DataTable/ItemGeneration/DT_AmmoProbability.DT_AmmoProbability" _array_element_3)
          (:`then`
            (set `local.SumPercent` (+ (`local.SumPercent`) (break `/Game/Blueprints/Datas/Struct/ItemGeneration/ST_ItemProbability` _returnvalue_3))))))
      (`BlueprintMapLibrary.Map_Add` (`local.ItemIdProbability`) "NewEnumerator2" (make `/Game/Blueprints/Datas/Struct/ItemGeneration/ST_ProbabilityInfo` (`local.SumPercent`) _outrownames_3)))
    (:`then_3`
      (set `local.SumPercent` 0)
      ; Health가 나올 확률 정보
      (bind _outrownames_4 (`DataTableFunctionLibrary.GetDataTableRowNames` "/Game/Blueprints/Datas/DataTable/ItemGeneration/DT_HelmatProbability.DT_HelmatProbability"))
      (for _array_element_4 _outrownames_4
        (bind _returnvalue_4 (`|GetDataTableRow` "/Game/Blueprints/Datas/DataTable/ItemGeneration/DT_HealthProbability.DT_HealthProbability" _array_element_4)
          (:`then`
            (set `local.SumPercent` (+ (`local.SumPercent`) (break `/Game/Blueprints/Datas/Struct/ItemGeneration/ST_ItemProbability` _returnvalue_4))))))
      (`BlueprintMapLibrary.Map_Add` (`local.ItemIdProbability`) "NewEnumerator3" (make `/Game/Blueprints/Datas/Struct/ItemGeneration/ST_ProbabilityInfo` (`local.SumPercent`) _outrownames_4)))
    (:`then_4`
      (set `local.SumPercent` 0)
      ; Boost가 나올 확률 정보
      (bind _outrownames_5 (`DataTableFunctionLibrary.GetDataTableRowNames` "/Game/Blueprints/Datas/DataTable/ItemGeneration/DT_BoostProbability.DT_BoostProbability"))
      (for _array_element_5 _outrownames_5
        (bind _returnvalue_5 (`|GetDataTableRow` "/Game/Blueprints/Datas/DataTable/ItemGeneration/DT_BoostProbability.DT_BoostProbability" _array_element_5)
          (:`then`
            (set `local.SumPercent` (+ (`local.SumPercent`) (break `/Game/Blueprints/Datas/Struct/ItemGeneration/ST_ItemProbability` _returnvalue_5))))))
      (`BlueprintMapLibrary.Map_Add` (`local.ItemIdProbability`) "NewEnumerator4" (make `/Game/Blueprints/Datas/Struct/ItemGeneration/ST_ProbabilityInfo` (`local.SumPercent`) _outrownames_5)))
    (:`then_5`
      (set `local.SumPercent` 0)
      ; Helmat이 나올 확률 정보
      (bind _outrownames_6 (`DataTableFunctionLibrary.GetDataTableRowNames` "/Game/Blueprints/Datas/DataTable/ItemGeneration/DT_HelmatProbability.DT_HelmatProbability"))
      (for _array_element_6 _outrownames_6
        (bind _returnvalue_6 (`|GetDataTableRow` "/Game/Blueprints/Datas/DataTable/ItemGeneration/DT_HelmatProbability.DT_HelmatProbability" _array_element_6)
          (:`then`
            (set `local.SumPercent` (+ (`local.SumPercent`) (break `/Game/Blueprints/Datas/Struct/ItemGeneration/ST_ItemProbability` _returnvalue_6))))))
      (`BlueprintMapLibrary.Map_Add` (`local.ItemIdProbability`) "NewEnumerator5" (make `/Game/Blueprints/Datas/Struct/ItemGeneration/ST_ProbabilityInfo` (`local.SumPercent`) _outrownames_6)))
    (:`then_6`
      (set `local.SumPercent` 0)
      ; Vest가 나올 확률 정보
      (bind _outrownames_7 (`DataTableFunctionLibrary.GetDataTableRowNames` "/Game/Blueprints/Datas/DataTable/ItemGeneration/DT_VestProbability.DT_VestProbability"))
      (for _array_element_7 _outrownames_7
        (bind _returnvalue_7 (`|GetDataTableRow` "/Game/Blueprints/Datas/DataTable/ItemGeneration/DT_VestProbability.DT_VestProbability" _array_element_7)
          (:`then`
            (set `local.SumPercent` (+ (`local.SumPercent`) (break `/Game/Blueprints/Datas/Struct/ItemGeneration/ST_ItemProbability` _returnvalue_7))))))
      (`BlueprintMapLibrary.Map_Add` (`local.ItemIdProbability`) "NewEnumerator6" (make `/Game/Blueprints/Datas/Struct/ItemGeneration/ST_ProbabilityInfo` (`local.SumPercent`) _outrownames_7)))
    (:`then_7`
      (set `local.SumPercent` 0)
      ; Backpack이 나올 확률 정보
      (bind _outrownames_8 (`DataTableFunctionLibrary.GetDataTableRowNames` "/Game/Blueprints/Datas/DataTable/ItemGeneration/DT_BackpacktProbability.DT_BackpacktProbability"))
      (for _array_element_8 _outrownames_8
        (bind _returnvalue_8 (`|GetDataTableRow` "/Game/Blueprints/Datas/DataTable/ItemGeneration/DT_BackpacktProbability.DT_BackpacktProbability" _array_element_8)
          (:`then`
            (set `local.SumPercent` (+ (`local.SumPercent`) (break `/Game/Blueprints/Datas/Struct/ItemGeneration/ST_ItemProbability` _returnvalue_8))))))
      (`BlueprintMapLibrary.Map_Add` (`local.ItemIdProbability`) "NewEnumerator7" (make `/Game/Blueprints/Datas/Struct/ItemGeneration/ST_ProbabilityInfo` (`local.SumPercent`) _outrownames_8)))
    (:`then_8`
      (set `local.SumPercent` 0)
      ; 무기장식품이 나올 확률 정보
      (bind _outrownames_9 (`DataTableFunctionLibrary.GetDataTableRowNames` "/Game/Blueprints/Datas/DataTable/ItemGeneration/DT_WeaponAccesseryProbability.DT_WeaponAccesseryProbability"))
      (for _array_element_9 _outrownames_9
        (bind _returnvalue_9 (`|GetDataTableRow` "/Game/Blueprints/Datas/DataTable/ItemGeneration/DT_WeaponAccesseryProbability.DT_WeaponAccesseryProbability" _array_element_9)
          (:`then`
            (set `local.SumPercent` (+ (`local.SumPercent`) (break `/Game/Blueprints/Datas/Struct/ItemGeneration/ST_ItemProbability` _returnvalue_9))))))
      (`BlueprintMapLibrary.Map_Add` (`local.ItemIdProbability`) "NewEnumerator1" (make `/Game/Blueprints/Datas/Struct/ItemGeneration/ST_ProbabilityInfo` (`local.SumPercent`) _outrownames_9)))
    (:`then_9`
      (set `local.SumPercent` 0)
      ; 무기가 나올 확률 정보
      (bind _outrownames_10 (`DataTableFunctionLibrary.GetDataTableRowNames` "/Game/Blueprints/Datas/DataTable/ItemGeneration/DT_WeaponProbability.DT_WeaponProbability"))
      (for _array_element_10 _outrownames_10
        (`|GetDataTableRow` "/Game/Blueprints/Datas/DataTable/ItemGeneration/DT_WeaponProbability.DT_WeaponProbability" _array_element_10
          (:`then`
            (set `local.SumPercent` (+ (`local.SumPercent`) 0)))))
      (`BlueprintMapLibrary.Map_Add` (`local.ItemIdProbability`) "NewEnumerator0" (make `/Game/Blueprints/Datas/Struct/ItemGeneration/ST_ProbabilityInfo` (`local.SumPercent`) _outrownames_10))
      ; DT 저장되어있는 위치값을 바탕으로 아이템 그룹 월드에 생성
      (bind _outrownames_11 (`DataTableFunctionLibrary.GetDataTableRowNames` "/Game/Blueprints/Datas/DataTable/ItemGeneration/DT_ItemGroupLocation.DT_ItemGroupLocation"))
      (for _array_element_11 _outrownames_11
        (bind _returnvalue_10 (`|GetDataTableRow` "/Game/Blueprints/Datas/DataTable/ItemGeneration/DT_ItemGroupLocation.DT_ItemGroupLocation" _array_element_11)
          (:`then`
            (bind _returnvalue_11 (`|SpawnActorFromClass` "/Game/Blueprints/Items/BP_ItemGroup.BP_ItemGroup_C" (`KismetMathLibrary.Conv_VectorToTransform` (break `/Game/Blueprints/Datas/Struct/ItemGeneration/ST_ItemGroupLocation` _returnvalue_10)) "AdjustIfPossibleButAlwaysSpawn" "MultiplyWithRoot" null null))
            (set `local.ItemGroupRef` _returnvalue_11)
            ; 생성될 아이템 갯수
            (bind _number (`self.RandomItemNumber` (`local.NumberProbability`)))
            (set `local.SpawnTransforms` (`/Game/Blueprints/Items/BP_ItemGroup.GetRandomTransforms` (`local.ItemGroupRef`) _number))
            (for _ (range 1 (+ _number 1))
              ; 랜덤 아이템 타입 정하기
              (bind _itemtype (`self.RandomItemType` (`local.ItemTypeProbability`) :!label _label))
              ; 아이템 타입 배열에 추가(중복없이)
              (if (== (`KismetArrayLibrary.Array_Find` (`local.ItemTypeArray`) _itemtype) -1)
                (`KismetArrayLibrary.Array_Add` (`local.ItemTypeArray`) _itemtype)
                (else
                  (goto _label))))
            (for _array_element_12 (`local.ItemTypeArray`)
              (bind _spawnitem (`self.RandomItemId` (`local.ItemIdProbability`) _array_element_12))
              (`KismetArrayLibrary.Array_Add` (`local.SpawnItemArray`) _spawnitem))
            (for (_array_element_13 _array_index) (`local.SpawnItemArray`)
              (set `local.ItemType` (break `/Game/Blueprints/Datas/Struct/ItemGeneration/ST_SpawnItem` _array_element_13))
              (set `local.SpawnId` (`.Id_5_B1043A264C668A363C8D1CA651E6AD28` (break `/Game/Blueprints/Datas/Struct/ItemGeneration/ST_SpawnItem` _array_element_13)))
              (bind _returnvalue_12 (`|SpawnActorFromClass` (select `/Game/Blueprints/Datas/Enum/Item/E_ItemType` (`local.ItemType`) :`NewEnumerator0` "/Game/Blueprints/Items/WorldItems/BP_WorldItem_Weapon.BP_WorldItem_Weapon_C" :`NewEnumerator1` "/Game/Blueprints/Items/WorldItems/BP_WorldItem_WeaponAccessery.BP_WorldItem_WeaponAccessery_C" :`NewEnumerator2` "/Game/Blueprints/Items/WorldItems/BP_WorldItem_Ammo.BP_WorldItem_Ammo_C" :`NewEnumerator3` "/Game/Blueprints/Items/WorldItems/BP_WorldItem_Health.BP_WorldItem_Health_C" :`NewEnumerator4` "/Game/Blueprints/Items/WorldItems/BP_WorldItem_Boost.BP_WorldItem_Boost_C" :`NewEnumerator5` "/Game/Blueprints/Items/WorldItems/BP_WorldItem_Helmet.BP_WorldItem_Helmet_C" :`NewEnumerator6` "/Game/Blueprints/Items/WorldItems/BP_WorldItem_Vest.BP_WorldItem_Vest_C" :`NewEnumerator7` "/Game/Blueprints/Items/WorldItems/BP_WorldItem_Backpack.BP_WorldItem_Backpack_C" :!type "/Game/Blueprints/Items/WorldItems/BP_WorldItemBase Class Reference") (`|GetArrayItem` (`local.SpawnTransforms`) _array_index) "AdjustIfPossibleButAlwaysSpawn" "MultiplyWithRoot" null (`local.SpawnId`) "1" null))
              (`/Game/Blueprints/Items/WorldItems/BP_WorldItemBase.InitSpawnData` _returnvalue_12 (`local.SpawnId`) "1"))
            (`KismetArrayLibrary.Array_Clear` (`local.ItemTypeArray`))
            (`KismetArrayLibrary.Array_Clear` (`local.SpawnItemArray`))))))))

(fn `RandomItemId`
  (params (ItemIdProbability :type "Map of /Game/Blueprints/Datas/Enum/Item/E_ItemType Enum to /Game/Blueprints/Datas/Struct/ItemGeneration/ST_ProbabilityInfo Structure") (ItemType :type "/Game/Blueprints/Datas/Enum/Item/E_ItemType Enum" :default "NewEnumerator0"))
  (returns (SpawnItem :type "/Game/Blueprints/Datas/Struct/ItemGeneration/ST_SpawnItem Structure"))
  (locals (ItemArr :type "Array of /Game/Blueprints/Datas/Struct/ItemGeneration/ST_SpawnItem Structure") (RandomValue :type Integer) (SumPercent :type Integer))
  (bind (_totalpercent _rownames) (break `/Game/Blueprints/Datas/Struct/ItemGeneration/ST_ProbabilityInfo` (`BlueprintMapLibrary.Map_Find` ItemIdProbability ItemType)))
  (set `local.RandomValue` (`KismetMathLibrary.RandomIntegerInRange` 1 _totalpercent))
  (for _array_element _rownames
    (bind _returnvalue (`|GetDataTableRow` (select `/Game/Blueprints/Datas/Enum/Item/E_ItemType` (`local.ItemType`) :`NewEnumerator0` "/Game/Blueprints/Datas/DataTable/ItemGeneration/DT_WeaponProbability.DT_WeaponProbability" :`NewEnumerator1` "/Game/Blueprints/Datas/DataTable/ItemGeneration/DT_WeaponAccesseryProbability.DT_WeaponAccesseryProbability" :`NewEnumerator2` "/Game/Blueprints/Datas/DataTable/ItemGeneration/DT_AmmoProbability.DT_AmmoProbability" :`NewEnumerator3` "/Game/Blueprints/Datas/DataTable/ItemGeneration/DT_HealthProbability.DT_HealthProbability" :`NewEnumerator4` "/Game/Blueprints/Datas/DataTable/ItemGeneration/DT_BoostProbability.DT_BoostProbability" :`NewEnumerator5` "/Game/Blueprints/Datas/DataTable/ItemGeneration/DT_HelmatProbability.DT_HelmatProbability" :`NewEnumerator6` "/Game/Blueprints/Datas/DataTable/ItemGeneration/DT_VestProbability.DT_VestProbability" :`NewEnumerator7` "/Game/Blueprints/Datas/DataTable/ItemGeneration/DT_BackpacktProbability.DT_BackpacktProbability" :!type "DataTable Object Reference") _array_element)
      (:`then`
        (bind _output_get (set `local.SumPercent` (+ (`local.SumPercent`) (`.Percent_2_7891DC5B471C477280BA8AB86C1EA68B` (break `/Game/Blueprints/Datas/Struct/ItemGeneration/ST_ItemProbability` _returnvalue)))))
        (if (>= _output_get (`local.RandomValue`))
          (return (make `/Game/Blueprints/Datas/Struct/ItemGeneration/ST_SpawnItem` (`local.ItemType`) _array_element)))))))

(fn `RandomItemNumber`
  (params (NumberPorbability :type "/Game/Blueprints/Datas/Struct/ItemGeneration/ST_ProbabilityInfo Structure"))
  (returns (Number :type Integer))
  (locals (NumberArr :type "Array of Integer") (TotalPercent :type Integer) (SumPercent :type Integer) (RandomValue :type Integer))
  (bind (_totalpercent _rownames) (break `/Game/Blueprints/Datas/Struct/ItemGeneration/ST_ProbabilityInfo` NumberPorbability))
  ; 아이템 몇개를 생성할 것인지
  (set `local.RandomValue` (`KismetMathLibrary.RandomIntegerInRange` 1 _totalpercent))
  (for _array_element _rownames
    (bind _returnvalue (`|GetDataTableRow` "/Game/Blueprints/Datas/DataTable/ItemGeneration/DT_NumberProbability.DT_NumberProbability" _array_element)
      (:`then`
        (bind _output_get (set `local.SumPercent` (+ (`local.SumPercent`) (`.Percent_10_98C4C114460AC2A5B6C6139E6052683E` (break `/Game/Blueprints/Datas/Struct/ItemGeneration/ST_NumberProbability` _returnvalue)))))
        (if (>= _output_get (`local.RandomValue`))
          (return (break `/Game/Blueprints/Datas/Struct/ItemGeneration/ST_NumberProbability` _returnvalue)))))))

(fn `RandomItemType`
  (params (ItemtypeProbability :type "/Game/Blueprints/Datas/Struct/ItemGeneration/ST_ProbabilityInfo Structure"))
  (returns (ItemType :type "/Game/Blueprints/Datas/Enum/Item/E_ItemType Enum"))
  (locals (ItemTypeArr :type "Array of /Game/Blueprints/Datas/Enum/Item/E_ItemType Enum") (TotalPercent :type Integer) (SumPercent :type Integer) (RandomValue :type Integer))
  (set `local.RandomValue` (`KismetMathLibrary.RandomIntegerInRange` 1 ItemtypeProbability_TotalPercent_3_2117AC6141EF372BDEDFF09957C672B2))
  (for _array_element ItemtypeProbability_RowNames_6_D024B5A8428702D861E663B43DCEE82A
    (bind _returnvalue (`|GetDataTableRow` "/Game/Blueprints/Datas/DataTable/ItemGeneration/DT_ItemTypeProbability.DT_ItemTypeProbability" _array_element)
      (:`then`
        (bind _output_get (set `local.SumPercent` (+ (`local.SumPercent`) (`.Percent_4_0DD76C4F406C51CD7E91A680B042B4A1` (break `/Game/Blueprints/Datas/Struct/ItemGeneration/ST_ItemTypeProbability` _returnvalue)))))
        (if (>= _output_get (`local.RandomValue`))
          (return (break `/Game/Blueprints/Datas/Struct/ItemGeneration/ST_ItemTypeProbability` _returnvalue)))))))

(fn `UserConstructionScript`)