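; BP_Player is the player character, handling movement, camera look, free look and pose/move states.
; Free look unlinks actor yaw from the controller and moves along actor yaw; on release, a timeline lerps control rotation back before relinking.
; Tick fires OnMovementStateChange only when squared velocity flips between moving and stopped.
; EvaluateMoveState uses ordered overwrites, giving aim priority over walk, then run, then default.
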(event `self.ReceiveTick`
  (params (DeltaSeconds :type "Float (single-precision)"))
  (bind _returnvalue (> (`KismetMathLibrary.VSizeSquared` (`self.GetVelocity`)) 0.0))
  (if (!= (`self.bIsMovingNow`) _returnvalue)
    (bind _output_get (set `self.bIsMovingNow` _returnvalue))
    (`self.OnMovementStateChange` _output_get)))

(event `OnFreeLookEnded`
  (bind (_direction _alpha) (`Timeline|Timeline` :!via `PlayFromStart`)
    (:`Update`
      (`Controller.SetControlRotation` (`self.GetController`) (`KismetMathLibrary.RLerp` (`self.FreeLookEndRotation`) (`self.FreeLookStartRotation`) _alpha true)))
    (:`Finished`
      (set `self.bUseControllerRotationYaw` true))))

(fn `EvaluateMoveState`
  ; 모든 조건 탐색 분기문
  (`|ExecutionSequence`
    (:`then_0`
      (set `self.CurrentMoveState` "NewEnumerator1"))
    (:`then_1`
      (if (`self.bIsRunPressed`)
        (set `self.CurrentMoveState` "NewEnumerator2")))
    (:`then_2`
      (if (`self.bIsWalkPressed`)
        (set `self.CurrentMoveState` "NewEnumerator0")))
    (:`then_3`
      (if (`self.bIsAimPressed`)
        (set `self.CurrentMoveState` "NewEnumerator3")))))

(fn `FreeLook`
  (params (bIsPressed :type Boolean))
  (bind _returnvalue (`self.GetControlRotation`))
  (if bIsPressed
    ; FreeLook 시작 회전값
    (set `self.FreeLookStartRotation` _returnvalue)
    (set `self.bUseControllerRotationYaw` false)
    (else
      ; FreeLook 끝 회전값
      (set `self.FreeLookEndRotation` _returnvalue)
      ; UseControllerRotationYaw True로 키는거 내부에 있음
      (`self.OnFreeLookEnded`))))

(fn `GetTargetRotationByControllerYaw`
  (returns (TargetRotation :type "Rotator Structure"))
  (return (`KismetMathLibrary.SelectRotator` (`/Game/Blueprints/Utils/MathUtils.GetYawOnlyRotation` (`self.GetControlRotation`)) (`/Game/Blueprints/Utils/MathUtils.GetYawOnlyRotation` (`self.K2_GetActorRotation`)) (`self.bUseControllerRotationYaw`))))

(fn `InputLookUp`
  (params (`Y Axis` :type "Float (double-precision)"))
  (`self.AddControllerPitchInput` `Y Axis`))

(fn `InputTurn`
  (params (`X Axis` :type "Float (double-precision)"))
  ; use controller Yaw를 true로 했기에
  ; 컨트롤러Yaw가 움직이는게 곧 플레이어Yaw가
  ; 움직이는 것이다
  (`self.AddControllerYawInput` `X Axis`))

(fn `Move`
  (params (bIsForward :type Boolean) (AxisValue :type "Float (double-precision)"))
  (bind _targetrotation (`self.GetTargetRotationByControllerYaw`))
  (if bIsForward
    (`self.AddMovementInput` (`KismetMathLibrary.GetForwardVector` _targetrotation) AxisValue)
    (else
      (`self.AddMovementInput` (`KismetMathLibrary.GetRightVector` _targetrotation) AxisValue))))

(fn `SetMaxWalkSpeed`
  (params (NewSpeed :type "Float (double-precision)"))
  (set `CharacterMovementComponent.MaxWalkSpeed` NewSpeed (`self.CharacterMovement`)))

(fn `UpdateMoveState`
  (params (NewState :type "/Game/Blueprints/Datas/Enum/E_MoveState Enum" :default "NewEnumerator0"))
  (set `self.CurrentMoveState` NewState))

(fn `UpdatePoseState`
  (params (NewPoseState :type "/Game/Blueprints/Datas/Enum/E_PoseState Enum" :default "NewEnumerator0"))
  (set `self.CurrentPoseState` NewPoseState))

(fn `UserConstructionScript`)