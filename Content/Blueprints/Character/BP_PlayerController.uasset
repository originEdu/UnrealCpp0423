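; Player controller that forwards move, look, jump, free-look and walk/run input to BP_Player and manages crouch and prone pose changes.
; Data tables resolve each pose transition and its duration, with a timer pausing movement input during timed transitions.
; Pose-keyed tables also set pitch limits and camera height, both eased by timelines.
; Walk speed follows armed, pose and move state, with separate values inside and outside a forward acceleration arc.
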(event `self.ReceiveTick`
  (params (DeltaSeconds :type "Float (single-precision)")))

(event `SetEnableMove`
  ; 키보드 포즈(alt, c, space) 인풋
  (set `self.bIsEnableMove` true))

(event `InputAction|Crouch`
  (params (Key :type "Key Structure"))
  (bind _playerref (`self.PlayerRef`))
  (bind (_transitiontime _topose) (`self.OnTransitionTimer` (`/Game/Blueprints/Character/BP_Player.bIsArmed` _playerref) "NewEnumerator1" (`/Game/Blueprints/Character/BP_Player.CurrentPoseState` _playerref)))
  ; 키보드 포즈(alt, c, space) 인풋
  (:`Pressed`
    (`self.UpdatePose` _transitiontime _topose)
    (`self.UpdatePitchLimit` (`/Game/Blueprints/Character/BP_Player.CurrentPoseState` (`self.PlayerRef`)) :!label _label)
    (`self.UpdateCameraHeight` false)
    (`self.UpdateWalkSpeed`)))

(event `self.ReceiveBeginPlay`
  ; Cast
  (bind _asbp_player (cast `/Game/Blueprints/Character/BP_Player` (`GameplayStatics.GetPlayerCharacter` 0)))
  (set `self.PlayerRef` _asbp_player)
  (`self.UpdatePitchLimit` "NewEnumerator0")
  (add `/Game/Blueprints/Character/BP_Player.OnMovementStateChange` (`self.PlayerRef`) (delegate `OnMoveMentStateChanged`)))

(event `OnMoveMentStateChanged`
  (params (bIsMovingNow :type Boolean))
  (`self.UpdateCameraHeight` bIsMovingNow))

(event `InputAction|Prone`
  (params (Key :type "Key Structure"))
  (bind _playerref (`self.PlayerRef`))
  (bind (_transitiontime _topose) (`self.OnTransitionTimer` (`/Game/Blueprints/Character/BP_Player.bIsArmed` _playerref) "NewEnumerator2" (`/Game/Blueprints/Character/BP_Player.CurrentPoseState` _playerref)))
  ; 키보드 포즈(alt, c, space) 인풋
  (:`Pressed`
    (`self.UpdatePose` _transitiontime _topose)
    (goto _label)))

(event `InputAxis|Turn`
  (params (AxisValue :type "Float (single-precision)"))
  ; 마우스 인풋
  (`/Game/Blueprints/Character/BP_Player.InputTurn` (`self.PlayerRef`) AxisValue))

(event `InputAxis|MoveForward`
  (params (AxisValue :type "Float (single-precision)"))
  ; 키보드 wasd 인풋
  (if (`self.bIsEnableMove`)
    (`/Game/Blueprints/Character/BP_Player.Move` (`self.PlayerRef`) true AxisValue)
    (`self.UpdateWalkSpeed`)))

(event `InputAxis|MoveRight`
  (params (AxisValue :type "Float (single-precision)"))
  ; 키보드 wasd 인풋
  (if (`self.bIsEnableMove`)
    (`/Game/Blueprints/Character/BP_Player.Move` (`self.PlayerRef`) false AxisValue)
    (`self.UpdateWalkSpeed`)))

(event `InputAxis|LookUp`
  (params (AxisValue :type "Float (single-precision)"))
  ; 마우스 인풋
  (if (`self.LimitPitchAngle` AxisValue)
    (`/Game/Blueprints/Character/BP_Player.InputLookUp` (`self.PlayerRef`) AxisValue)))

(event `InputAction|Jump`
  (params (Key :type "Key Structure"))
  (bind _playerref (`self.PlayerRef`))
  (bind _currentposestate (`/Game/Blueprints/Character/BP_Player.CurrentPoseState` _playerref))
  (bind (_transitiontime _topose) (`self.OnTransitionTimer` (`/Game/Blueprints/Character/BP_Player.bIsArmed` _playerref) "NewEnumerator0" _currentposestate))
  ; 키보드 포즈(alt, c, space) 인풋
  (:`Pressed`
    (if (`|EnumEquality` _currentposestate "NewEnumerator0")
      (`Character.Jump` (`self.PlayerRef`))
      (else
        (`self.UpdatePose` _transitiontime _topose)
        (goto _label)))))

(event `InputAction|FreeLook`
  (params (Key :type "Key Structure"))
  (bind _playerref (`self.PlayerRef`))
  ; 자유시점
  (:`Pressed`
    (`/Game/Blueprints/Character/BP_Player.FreeLook` _playerref true))
  (:`Released`
    (`/Game/Blueprints/Character/BP_Player.FreeLook` _playerref false)))

(event `InputAction|Walk`
  (params (Key :type "Key Structure"))
  (bind _playerref (`self.PlayerRef`))
  ; 걷기와 뛰기
  (:`Pressed`
    (set `/Game/Blueprints/Character/BP_Player.bIsWalkPressed` true _playerref)
    (`/Game/Blueprints/Character/BP_Player.EvaluateMoveState` _playerref :!label _label_2)
    (`self.UpdateWalkSpeed`))
  (:`Released`
    (set `/Game/Blueprints/Character/BP_Player.bIsWalkPressed` false _playerref)
    (goto _label_2)))

(event `InputAction|Run`
  (params (Key :type "Key Structure"))
  (bind _playerref (`self.PlayerRef`))
  ; 걷기와 뛰기
  (:`Pressed`
    (set `/Game/Blueprints/Character/BP_Player.bIsRunPressed` true _playerref)
    (`/Game/Blueprints/Character/BP_Player.EvaluateMoveState` _playerref :!label _label_3)
    (`self.UpdateWalkSpeed`))
  (:`Released`
    (set `/Game/Blueprints/Character/BP_Player.bIsRunPressed` false _playerref)
    (goto _label_3)))

(event `MoveToLimitAngle`
  (params (LimitPitch :type "Float (double-precision)") (CharacterRotation :type "Rotator Structure"))
  (bind (_direction _alpha) (`Timeline|TL_MoveToLimitAngle` :!via `PlayFromStart`)
    (:`Update`
      (`self.SetControlRotation` (`KismetMathLibrary.RLerp` CharacterRotation (`KismetMathLibrary.MakeRotator` (.roll CharacterRotation) LimitPitch (.yaw CharacterRotation)) _alpha true)))))

(event `ChangeCameraHeight`
  (params (TargetHeight :type "Float (double-precision)") (CurrentHeight :type "Float (double-precision)"))
  (bind _springarm (`/Game/Blueprints/Character/BP_Player.SpringArm` (`self.PlayerRef`)))
  (bind (_socketoffset_x _socketoffset_y) (`KismetMathLibrary.BreakVector` (`SpringArmComponent.SocketOffset` _springarm)))
  (bind (_direction _alpha) (`Timeline|TL_ChangeCameraHeight` :!via `PlayFromStart`)
    (:`Update`
      (set `SpringArmComponent.SocketOffset` (`KismetMathLibrary.MakeVector` _socketoffset_x _socketoffset_y (`KismetMathLibrary.Lerp` CurrentHeight TargetHeight _alpha)) _springarm))))

(fn `IsAcceleratingForwordArc`
  (returns (bIsForward :type Boolean))
  (bind _playerref (`self.PlayerRef`))
  (return (>= (`KismetMathLibrary.Dot_VectorVector` (`self.GetActorForwardVector` _playerref) (`KismetMathLibrary.Normal` (`CharacterMovementComponent.GetCurrentAcceleration` (`Character.CharacterMovement` _playerref)))) 0.707)))

(fn `LimitPitchAngle`
  (params (Axis :type "Float (double-precision)"))
  (returns (ReturnValue :type Boolean))
  (bind (_returnvalue_roll _returnvalue_pitch) (`KismetMathLibrary.BreakRotator` (`self.GetControlRotation`)))
  (bind _returnvalue (+ _returnvalue_pitch (* (`local.Axis`) (`self.GetDeprecatedInputPitchScale`))))
  (return (or (> _returnvalue (`self.CachedBottomLimit`)) (< _returnvalue (`self.CachedTopLimit`)))))

(fn `OnTransitionTimer`
  (params (bIsArmed :type Boolean) (TargetPose :type "/Game/Blueprints/Datas/Enum/E_PoseState Enum" :default "NewEnumerator0") (FromPose :type "/Game/Blueprints/Datas/Enum/E_PoseState Enum" :default "NewEnumerator0"))
  (returns (TransitionTime :type "Float (double-precision)") (ToPose :type "/Game/Blueprints/Datas/Enum/E_PoseState Enum"))
  (locals (ReturnPose :type "/Game/Blueprints/Datas/Enum/E_PoseState Enum" :default "NewEnumerator0"))
  (set `local.ReturnPose` (`self.TryGetPoseTransition` TargetPose FromPose))
  (bind _returnvalue (`|GetDataTableRow` "/Game/Blueprints/Datas/DataTable/DT_ProneTime.DT_ProneTime" (`KismetStringLibrary.Conv_StringToName` (`KismetStringLibrary.Concat_StrStr` (`KismetStringLibrary.Conv_BoolToString` bIsArmed) "_" (`|GetEnumeratorNameAsString` (`local.FromPose`)) "_" (`|GetEnumeratorNameAsString` (`local.ReturnPose`)))))
    (:`then`
      _)
    (:`RowNotFound`
      _))
  (return (break `/Game/Blueprints/Datas/Struct/ST_ProneTime` _returnvalue) (`local.ReturnPose`)))

(fn `TryGetPoseTransition`
  (params (TargetPose :type "/Game/Blueprints/Datas/Enum/E_PoseState Enum" :default "NewEnumerator0") (FromPose :type "/Game/Blueprints/Datas/Enum/E_PoseState Enum" :default "NewEnumerator0"))
  (returns (ToPose :type "/Game/Blueprints/Datas/Enum/E_PoseState Enum"))
  (bind _returnvalue (`|GetDataTableRow` "/Game/Blueprints/Datas/DataTable/DT_PoseTransition.DT_PoseTransition" (`KismetStringLibrary.Conv_StringToName` (`KismetStringLibrary.Concat_StrStr` (`|GetEnumeratorNameAsString` TargetPose) "_" (`|GetEnumeratorNameAsString` FromPose))))
    (:`then`
      _)
    (:`RowNotFound`
      _))
  (return (break `/Game/Blueprints/Datas/Struct/ST_PoseTransition` _returnvalue)))

(fn `UpdateCameraHeight`
  (params (bIsMovingNow :type Boolean))
  (locals (CurrentPose :type String) (RowName :type String))
  (bind _currentposestate (`/Game/Blueprints/Character/BP_Player.CurrentPoseState` (`self.PlayerRef`)))
  (bind (_socketoffset_x _socketoffset_y _socketoffset_z) (`KismetMathLibrary.BreakVector` (`SpringArmComponent.SocketOffset` (`/Game/Blueprints/Character/BP_Player.SpringArm` (`self.PlayerRef`)))))
  (`|ExecutionSequence`
    (:`then_0`
      (set `local.CurrentPose` (`|GetEnumeratorNameAsString` _currentposestate))
      (if (`|EnumInequality` _currentposestate "NewEnumerator1")
        (set `local.RowName` (`local.CurrentPose`))
        (else
          (set `local.RowName` (`local.CurrentPose`))
          (if (`local.bIsMovingNow`)
            (set `local.RowName` (`KismetStringLibrary.Concat_StrStr` (`local.CurrentPose`) "_" (`KismetStringLibrary.Conv_BoolToString` (`/Game/Blueprints/Character/BP_Player.bIsArmed` (`self.PlayerRef`))) "_Move"))))))
    (:`then_1`
      (bind _returnvalue (`|GetDataTableRow` "/Game/Blueprints/Datas/DataTable/DT_CameraHeight.DT_CameraHeight" (`KismetStringLibrary.Conv_StringToName` (`local.RowName`)))
        (:`then`
          (`self.ChangeCameraHeight` (break `/Game/Blueprints/Datas/Struct/ST_CameraHeight` _returnvalue) _socketoffset_z))))))

(fn `UpdatePitchLimit`
  (params (ToPose :type "/Game/Blueprints/Datas/Enum/E_PoseState Enum" :default "NewEnumerator0"))
  (locals (ControlRotation :type "Rotator Structure" :default (struct)))
  (bind (_returnvalue_roll _returnvalue_pitch) (`KismetMathLibrary.BreakRotator` (`self.GetControlRotation`)))
  (bind _controlrotation (`local.ControlRotation`))
  (`|ExecutionSequence`
    (:`then_0`
      (bind _returnvalue (`|GetDataTableRow` "/Game/Blueprints/Datas/DataTable/DT_PitchLimit.DT_PitchLimit" (`KismetStringLibrary.Conv_StringToName` (`|GetEnumeratorNameAsString` ToPose)))
        (:`then`
          (`|ExecutionSequence`
            (:`then_0`
              (set `self.CachedTopLimit` (break `/Game/Blueprints/Datas/Struct/ST_PitchLimit` _returnvalue)))
            (:`then_1`
              (set `self.CachedBottomLimit` (`.BottomLimit_5_BB4214FA41D529A07A14D5B686BA9C76` (break `/Game/Blueprints/Datas/Struct/ST_PitchLimit` _returnvalue))))))))
    (:`then_1`
      (set `local.ControlRotation` (`self.GetControlRotation`))
      (if (or (> _returnvalue_pitch (`self.CachedBottomLimit`)) (< _returnvalue_pitch (`self.CachedTopLimit`)))
        _
        (elif (< (`KismetMathLibrary.Abs` (- _returnvalue_pitch (`self.CachedTopLimit`))) (`KismetMathLibrary.Abs` (- _returnvalue_pitch (`self.CachedBottomLimit`))))
          (`self.MoveToLimitAngle` (`self.CachedTopLimit`) _controlrotation)
          (else
            (`self.MoveToLimitAngle` (`self.CachedBottomLimit`) _controlrotation)))))))

(fn `UpdatePose`
  (params (WaitTime :type "Float (double-precision)") (ToPose :type "/Game/Blueprints/Datas/Enum/E_PoseState Enum" :default "NewEnumerator0"))
  (if (!= WaitTime 0.0)
    (set `self.bIsEnableMove` false)
    (`KismetSystemLibrary.K2_SetTimerDelegate` (`|CreateDelegate` :!event `SetEnableMove`) WaitTime))
  (`/Game/Blueprints/Character/BP_Player.UpdatePoseState` (`self.PlayerRef`) ToPose))

(fn `UpdateWalkSpeed`
  (locals (RowName :type String) (OutRow :type "/Game/Blueprints/Datas/Struct/ST_WalkSpeed Structure"))
  ; RowName 세팅
  (`|ExecutionSequence`
    (:`then_0`
      (set `local.RowName` (`KismetStringLibrary.Conv_BoolToString` (`/Game/Blueprints/Character/BP_Player.bIsArmed` (`self.PlayerRef`)))))
    (:`then_1`
      (bind _output_get (set `local.RowName` (`KismetStringLibrary.Concat_StrStr` (`local.RowName`) "_" (`|GetEnumeratorNameAsString` (`/Game/Blueprints/Character/BP_Player.CurrentPoseState` (`self.PlayerRef`))))))
      ; 현재 Move상태에 따른 MaxSpeed 세팅
      (bind _returnvalue (`|GetDataTableRow` "/Game/Blueprints/Datas/DataTable/DT_WalkSpeed.DT_WalkSpeed" (`KismetStringLibrary.Conv_StringToName` _output_get))
        (:`then`
          (bind _output_get_2 (set `local.OutRow` _returnvalue))
          (bind (_returnvalue_forwardspeed _returnvalue_nonforwardspeed) (break `/Game/Blueprints/Datas/Struct/ST_DirectionalSpeed` (select `/Game/Blueprints/Datas/Enum/E_MoveState` (`/Game/Blueprints/Character/BP_Player.CurrentMoveState` (`self.PlayerRef`)) :`NewEnumerator0` (break `/Game/Blueprints/Datas/Struct/ST_WalkSpeed` _output_get_2) :`NewEnumerator1` (`.Jog_9_DD5102BF49907DBC6E358A9AE6345CC8` (break `/Game/Blueprints/Datas/Struct/ST_WalkSpeed` _output_get_2)) :`NewEnumerator2` (`.Run_10_44E90D2C4F89973EC19E45948617B3D4` (break `/Game/Blueprints/Datas/Struct/ST_WalkSpeed` _output_get_2)) :`NewEnumerator3` (`.Aim_11_06322F3143BC385937A45684BB8B591A` (break `/Game/Blueprints/Datas/Struct/ST_WalkSpeed` _output_get_2)))))
          (`/Game/Blueprints/Character/BP_Player.SetMaxWalkSpeed` (`self.PlayerRef`) (`KismetMathLibrary.SelectFloat` _returnvalue_forwardspeed _returnvalue_nonforwardspeed (`self.IsAcceleratingForwordArc`))))))))

(fn `UserConstructionScript`)